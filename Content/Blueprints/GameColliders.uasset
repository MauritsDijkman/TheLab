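; GameColliders shows level completion by recoloring a set of glass meshes to green once the player has won.
; Every Tick, the CheckLevel1 flag selects whether it reads Level1Won or Level2Won from the Character reference.
; It then loops over MeshToChange, setting the first material slot to M_Glass_Green when won or M_Glass otherwise.
; The state is polled and reapplied each frame rather than driven by events.
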(event `self.ReceiveTick`
  (params (DeltaSeconds :type "Float (single-precision)"))
  ;[1 1 1] Check Which To Check
  (if (`self.CheckLevel1`)
    ;[1 1 1] Check Level 1
    (if (`PlayerCharacter.level1Won` (`self.Character`))
      ;[1 1 1] Loop And Change To Finished Material
      (for _array_element (`self.MeshToChange`) :!label _label
        (`PrimitiveComponent.SetMaterial` (`StaticMeshActor.StaticMeshComponent` _array_element) 0 "/Game/Material/M_Glass_Green.M_Glass_Green"))
      (else
        ;[1 1 1] Loop And Change To Original Material
        (for _array_element_2 (`self.MeshToChange`) :!label _label_2
          (`PrimitiveComponent.SetMaterial` (`StaticMeshActor.StaticMeshComponent` _array_element_2) 0 "/Game/StarterContent/Materials/M_Glass.M_Glass"))))
    (else
      ;[1 1 1] Check Level 2
      (if (`PlayerCharacter.level2Won` (`self.Character`))
        (goto _label)
        (else
          (goto _label_2))))))

(fn `UserConstructionScript`)