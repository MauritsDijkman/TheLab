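; Door actor that swings open for the player only once both Level 1 and Level 2 are won.
; A trigger box checks the overlapping PlayerCharacter_BP's win flags and plays the Door timeline, which scales an Angle variable to set the door mesh's relative yaw.
; The timeline reverses when the player leaves the box, without checking the flags.
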(event `self.Box.OnComponentBeginOverlap`
  (params (OverlappedComponent :type "PrimitiveComponent Object Reference") (OtherActor :type "Actor Object Reference") (OtherComp :type "PrimitiveComponent Object Reference") (OtherBodyIndex :type Integer) (bFromSweep :type Boolean) (SweepResult :type "HitResult Structure (by ref)"))
  ;[1 1 1] On Begin Overlap
  (bind _asplayer_character_bp (cast `/Game/Blueprints/Characters/PlayerCharacter_BP` OtherActor))
  (if (`PlayerCharacter.level2Won` _asplayer_character_bp)
    (if (`PlayerCharacter.level1Won` _asplayer_character_bp)
      ;[1 1 1] Animate Door
      (bind (_direction _newtrack_0) (`Timeline|Door` :!label _label)
        (:`Update`
          (`SceneComponent.K2_SetRelativeRotation` (`self.SM_Door`) (`KismetMathLibrary.MakeRotator` 0.0 0.0 (* _newtrack_0 (`self.Angle`))) false false))))))

(event `self.Box.OnComponentEndOverlap`
  (params (OverlappedComponent :type "PrimitiveComponent Object Reference") (OtherActor :type "Actor Object Reference") (OtherComp :type "PrimitiveComponent Object Reference") (OtherBodyIndex :type Integer))
  ;[1 1 1] On End Overlap
  (cast `/Game/Blueprints/Characters/PlayerCharacter_BP` OtherActor)
  (goto _label :!via `Reverse`))

(fn `UserConstructionScript`)