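; Player character for a maze game that tracks completion of two levels and persists it through a StatsSave save game slot.
; BeginPlay clears the fade-out flag and loads progress; SaveGame writes it back, reusing or creating the slot's save object.
; SetFadeOut sets the flag that makes Tick call CallFadeOut every frame.
; Pressing Escape deletes the save slot and quits, so manually exiting wipes progress.
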(event `self.ReceiveBeginPlay`
  ;[1 1 1] Start
  (`|ExecutionSequence`
    (:`then_0`
      (set `self.StartFadeOut` false))
    (:`then_1`
      (`self.LoadGame` (`self.Slot Name Save`)))))

(event `Key|Escape`
  (params (Key :type "Key Structure"))
  ;[1 1 1] Handle Escape Pressed
  (:`Pressed`
    (`GameplayStatics.DeleteGameInSlot` (`self.Slot Name Save`))
    (`KismetSystemLibrary.QuitGame` null "Quit")))

(event `self.ReceiveTick`
  (params (DeltaSeconds :type "Float (single-precision)"))
  ;[1 1 1] Handle Fade Out
  (if (`self.StartFadeOut`)
    (`self.FadeOut`)))

(fn `LoadGame`
  (params (SlotName :type String :default "Slot1"))
  ;[1 1 1] Load Game Data From PC
  (bind _returnvalue (`GameplayStatics.DoesSaveGameExist` SlotName))
  (if _returnvalue
    (bind _returnvalue_2 (`GameplayStatics.LoadGameFromSlot` (`local.SlotName`)))
    (bind _asstats_save (cast `/Game/Blueprints/StatsSave` _returnvalue_2))
    (set `self.level1Won` (`/Game/Blueprints/StatsSave.Level1Finished` _asstats_save))
    (set `self.level2Won` (`/Game/Blueprints/StatsSave.Level2Finished` _asstats_save))))

(fn `SaveGame`
  (params (SlotName :type String :default "Slot1"))
  ;[1 1 1] Save Game Data To PC
  (bind _returnvalue (`GameplayStatics.DoesSaveGameExist` SlotName))
  (if _returnvalue
    (bind _returnvalue_2 (`GameplayStatics.LoadGameFromSlot` (`local.SlotName`)))
    (set `self.SaveRef` _returnvalue_2)
    (else
      (bind _returnvalue_3 (`GameplayStatics.CreateSaveGameObject` "/Game/Blueprints/StatsSave.StatsSave_C"))
      (bind _output_get (set `self.SaveRef` _returnvalue_3))))
  (bind _asstats_save (cast `/Game/Blueprints/StatsSave` _output_get))
  (set `/Game/Blueprints/StatsSave.Level1Finished` (`self.level1Won`) _asstats_save)
  (set `/Game/Blueprints/StatsSave.Level2Finished` (`self.level2Won`) _asstats_save)
  (`GameplayStatics.SaveGameToSlot` (`self.SaveRef`) (`local.SlotName`)))

(fn `SetFadeOut`
  (params (StartingFadeOut :type Boolean))
  ;[1 1 1] Set Fade Out Variable
  (set `self.StartFadeOut` StartingFadeOut))

(fn `UserConstructionScript`)